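; BP_Enemy is a killing-floor enemy that chases the VR player.
; On BeginPlay it registers itself in the game mode's remaining-enemy count and uses AIMoveTo to pursue the player character.
; When its capsule overlaps the player, it decrements that count, has the game mode check how many enemies are left, and destroys itself.
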(event `self.ReceiveBeginPlay`
  (bind _asbp_killing_floor_game_mode_base (cast `/Game/Blueprints/BP_KillingFloorGameModeBase` (`GameplayStatics.GetGameMode`)))
  (`KillingFloorGameModeBase.AddCurrentEnemyLeft` _asbp_killing_floor_game_mode_base)
  (bind _asbp_vrplayer (cast `/Game/Blueprints/BP_VRPlayer` (`GameplayStatics.GetPlayerCharacter` 0)))
  (`|AIMoveTo` self (0.0 0.0 0.0) _asbp_vrplayer))

(event `self.CapsuleComponent.OnComponentBeginOverlap`
  (params (OverlappedComponent :type "PrimitiveComponent Object Reference") (OtherActor :type "Actor Object Reference") (OtherComp :type "PrimitiveComponent Object Reference") (OtherBodyIndex :type Integer) (bFromSweep :type Boolean) (SweepResult :type "HitResult Structure (by ref)"))
  (cast `/Game/Blueprints/BP_VRPlayer` OtherActor)
  (bind _asbp_killing_floor_game_mode_base (cast `/Game/Blueprints/BP_KillingFloorGameModeBase` (`GameplayStatics.GetGameMode`)))
  (`KillingFloorGameModeBase.SubtractCurrentEnemyLeft` _asbp_killing_floor_game_mode_base)
  (`KillingFloorGameModeBase.CheckEnemyLeft` _asbp_killing_floor_game_mode_base)
  (`self.K2_DestroyActor`))

(fn `UserConstructionScript`)