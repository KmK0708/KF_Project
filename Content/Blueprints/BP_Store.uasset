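; BP_Store is a shop actor in a VR game that opens a store menu when the player enters its collision area.
; On overlap by the player character, it sets the in-shop flag on BP_VRPlayer, waits briefly, then spawns BP_StoreMenu at a hard-coded world location and hands it a self-reference.
; Disconnected nodes for a viewport widget shop with camera switch and mouse cursor remain in the graph but never run.
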(event `self.ReceiveActorBeginOverlap`
  (params (OtherActor :type "Actor Object Reference")))

(event `self.StoreOverlapCollision.OnComponentBeginOverlap`
  (params (OverlappedComponent :type "PrimitiveComponent Object Reference") (OtherActor :type "Actor Object Reference") (OtherComp :type "PrimitiveComponent Object Reference") (OtherBodyIndex :type Integer) (bFromSweep :type Boolean) (SweepResult :type "HitResult Structure (by ref)"))
  (bind _returnvalue (`GameplayStatics.GetPlayerCharacter` 0))
  (if (== OtherActor _returnvalue)
    (bind _asbp_vrplayer (cast `/Game/Blueprints/BP_VRPlayer` _returnvalue))
    (set `VRPlayer.bisShopIn` true _asbp_vrplayer)
    (`KismetSystemLibrary.Delay` 1.0)
    (bind _returnvalue_2 (`|SpawnActorFromClass` "/Game/Blueprints/WB/BP_StoreMenu.BP_StoreMenu_C" (`KismetMathLibrary.MakeTransform` (-2090.0 90.0 100.0)) "Undefined" "OverrideRootScale" null null))
    (set `/Game/Blueprints/WB/BP_StoreMenu.StoreM` self _returnvalue_2)))

(fn `UserConstructionScript`)