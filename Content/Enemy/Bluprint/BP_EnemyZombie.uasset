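; BP_EnemyZombie is a zombie enemy Blueprint that registers itself with the wave's remaining-enemy count in BP_KillingFloorGameModeBase.
; On BeginPlay it casts the game mode and calls AddCurrentEnemyLeft.
; Disconnected nodes hold an unused removal path that decrements the count, checks enemies left and destroys the actor, plus a debug print of the Fsm state.
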(event `self.ReceiveBeginPlay`
  (bind _asbp_killing_floor_game_mode_base (cast `/Game/Blueprints/BP_KillingFloorGameModeBase` (`GameplayStatics.GetGameMode`)))
  (`KillingFloorGameModeBase.AddCurrentEnemyLeft` _asbp_killing_floor_game_mode_base))

(event `self.ReceiveTick`
  (params (DeltaSeconds :type "Float (single-precision)")))

(fn `UserConstructionScript`)